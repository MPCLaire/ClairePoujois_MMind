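; BP_NPC is an AI-driven NPC with shoot and punch actions and a cover-point search.
; Shoot turns the capsule toward the player; Attack pauses movement through AB_NPC.
; Both set a state enum, wait a second, then clear their AIC_NPC blackboard flag and reset the state.
; Despite its name, FindNearestCover returns the farthest cover point's location, since it keeps the larger distance, with debug prints along the way.
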(event `self.ReceiveBeginPlay`)

(event `Shoot`
  (`SceneComponent.K2_SetWorldRotation` (`self.CapsuleComponent`) (`KismetMathLibrary.FindLookAtRotation` (`self.K2_GetActorLocation`) (`self.K2_GetActorLocation` (`GameplayStatics.GetPlayerCharacter` 0))) false false)
  (set `self.Enum` "NewEnumerator1")
  (bind _asaic_npc (cast `/Game/IA/AIC_NPC` (`AIBlueprintHelperLibrary.GetAIController` self)))
  (`KismetSystemLibrary.Delay` 1.0)
  (`BlackboardComponent.SetValueAsBool` (`AIController.Blackboard` _asaic_npc) (`self.CanShoot`) false)
  (set `self.Enum` "NewEnumerator0"))

(event `Attack`
  (set `self.Enum` "NewEnumerator2")
  (bind _asab_npc (cast `/Game/Animation/AB_NPC` (`SkeletalMeshComponent.GetAnimInstance` (`self.Mesh`))))
  (set `/Game/Animation/AB_NPC.CanMove?` false _asab_npc)
  (bind _asaic_npc (cast `/Game/IA/AIC_NPC` (`AIBlueprintHelperLibrary.GetAIController` self)))
  (`KismetSystemLibrary.Delay` 1.0)
  (`BlackboardComponent.SetValueAsBool` (`AIController.Blackboard` _asaic_npc) (`self.CanPunch`) false)
  (set `self.Enum` "NewEnumerator0")
  (set `/Game/Animation/AB_NPC.CanMove?` true _asab_npc))

(fn `FindNearestCover`
  (returns (ClosestLocation :type "Vector Structure"))
  (bind _closestindex (`self.ClosestIndex`))
  (`KismetSystemLibrary.PrintString` "Hello")
  (set `self.ClosestDistance` 0.0)
  (for (_array_element _array_index) (`self.CoverpointsList`)
    (bind _returnvalue (`KismetMathLibrary.VSize` (- (`self.K2_GetActorLocation` _array_element) (`self.K2_GetActorLocation`))))
    (if (> _returnvalue (`self.ClosestDistance`))
      (set `self.ClosestDistance` _returnvalue)
      (bind _output_get (set `self.ClosestIndex` _array_index))
      (`KismetSystemLibrary.PrintString` (`KismetStringLibrary.Conv_IntToString` _output_get) true true (struct :`R` 1.0 :`G` 0.982222 :`A` 1.0))))
  (`KismetSystemLibrary.PrintString` (`KismetStringLibrary.Conv_IntToString` _closestindex) true true (struct :`R` 1.0 :`B` 0.707057 :`A` 1.0))
  (set `self.ActualCover` (`self.ClosestDistance`))
  (return (`self.K2_GetActorLocation` (`|GetArrayItem` (`self.CoverpointsList`) _closestindex))))

(fn `UserConstructionScript`)